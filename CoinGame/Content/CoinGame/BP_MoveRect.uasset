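; BP_MoveRect is a CoinGame actor that moves its Cube component around a 100-unit square in the local X-Z plane.
; Each Tick switches on MoveType, shifts X or Z by one unit, and advances to the next state at the edge's limit.
; The step ignores delta time, so speed depends on frame rate.
; State names are offset from motion: Down decreases X and Left decreases Z.
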(event EventBeginPlay)

(event Collision|EventActorBeginOverlap
  (params (OtherActor :type Actor%20Object%20Reference)))

(event EventTick
  (params (DeltaSeconds :type Float%20%28single-precision%29))
  (switch Utilities|FlowControl|Switch|SwitchonEN_MoveType (Variables|Default|GetMoveType)
    (:NewEnumerator0
      (bind _output_get (Variables|Default|SetLocation%20X (+ (Variables|Default|GetLocation%20X) 1.0)))
      (Transformation|SetRelativeLocation (Variables|Default|GetCube) (Math|Vector|MakeVector _output_get 0.0 (Variables|Default|GetLocation%20Z)) false false)
      (if (>= (.x (Variables|/Script/Engine.SceneComponent|GetRelativeLocation (Variables|Default|GetCube))) 1e+02)
        (Variables|Default|SetMoveType "NewEnumerator1")))
    (:NewEnumerator1
      (bind _output_get_2 (Variables|Default|SetLocation%20Z (+ (Variables|Default|GetLocation%20Z) 1.0)))
      (Transformation|SetRelativeLocation (Variables|Default|GetCube) (Math|Vector|MakeVector (Variables|Default|GetLocation%20X) 0.0 _output_get_2) false false)
      (if (>= (.z (Variables|/Script/Engine.SceneComponent|GetRelativeLocation (Variables|Default|GetCube))) 1e+02)
        (Variables|Default|SetMoveType "NewEnumerator2")))
    (:NewEnumerator2
      (bind _output_get_3 (Variables|Default|SetLocation%20X (+ (Variables|Default|GetLocation%20X) -1.0)))
      (Transformation|SetRelativeLocation (Variables|Default|GetCube) (Math|Vector|MakeVector _output_get_3 0.0 (Variables|Default|GetLocation%20Z)) false false)
      (if (<= (.x (Variables|/Script/Engine.SceneComponent|GetRelativeLocation (Variables|Default|GetCube))) 0.0)
        (Variables|Default|SetMoveType "NewEnumerator3")))
    (:NewEnumerator3
      (bind _output_get_4 (Variables|Default|SetLocation%20Z (+ (Variables|Default|GetLocation%20Z) -1.0)))
      (Transformation|SetRelativeLocation (Variables|Default|GetCube) (Math|Vector|MakeVector (Variables|Default|GetLocation%20X) 0.0 _output_get_4) false false)
      (if (<= (.z (Variables|/Script/Engine.SceneComponent|GetRelativeLocation (Variables|Default|GetCube))) 0.0)
        (Variables|Default|SetMoveType "NewEnumerator0")))))

(fn ConstructionScript)